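; Special checkpoint marker that reveals itself to the BlueROV and adds to its SpecialCheckpointCount.
; Its sphere and two glow components start hidden and show only while a BP_BlueRov overlaps the Box trigger.
; Actor overlap with a Player-tagged actor increments the count on the player pawn.
; Leaving the box hides the marker, then after a delay increments the count again and destroys the actor.
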(event `self.ReceiveBeginPlay`
  (`self.ChangeComponentVisibility` false))

(event `ChangeComponentVisibility`
  (params (`Visible?` :type Boolean))
  ;[1 1 1] condition check for change in visibility
  (`SceneComponent.SetVisibility` (`self.Sphere`) `Visible?` false)
  (`SceneComponent.SetVisibility` (`self.glow`) `Visible?` false)
  (`SceneComponent.SetVisibility` (`self.glow1`) `Visible?` false)
  (`SceneComponent.SetHiddenInGame` (`self.glow`) true true :!enabledstate Disabled)
  (`SceneComponent.SetHiddenInGame` (`self.Sphere`) true true :!enabledstate Disabled)
  (`SceneComponent.SetHiddenInGame` (`self.glow1`) true true :!enabledstate Disabled))

(event `self.Box.OnComponentBeginOverlap`
  (params (OverlappedComponent :type "PrimitiveComponent Object Reference") (OtherActor :type "Actor Object Reference") (OtherComp :type "PrimitiveComponent Object Reference") (OtherBodyIndex :type Integer) (bFromSweep :type Boolean) (SweepResult :type "HitResult Structure (by ref)"))
  ;[1 1 1] change in visibility based on trigger box
  (cast `/Game/Blueprints/BP_BlueRov` OtherActor)
  (`self.ChangeComponentVisibility` true))

(event `self.Box.OnComponentEndOverlap`
  (params (OverlappedComponent :type "PrimitiveComponent Object Reference") (OtherActor :type "Actor Object Reference") (OtherComp :type "PrimitiveComponent Object Reference") (OtherBodyIndex :type Integer))
  ;[1 1 1] change in visibility based on trigger box
  (bind _asbp_blue_rov (cast `/Game/Blueprints/BP_BlueRov` OtherActor))
  (`self.ChangeComponentVisibility` false)
  (`KismetSystemLibrary.Delay` 25.0)
  (set `/Game/Blueprints/BP_BlueRov.SpecialCheckpointCount` (+ (`/Game/Blueprints/BP_BlueRov.SpecialCheckpointCount` _asbp_blue_rov) 1) _asbp_blue_rov)
  (`self.K2_DestroyActor`))

(event `self.ReceiveActorBeginOverlap` :!enabledstate Disabled
  (params (OtherActor :type "Actor Object Reference"))
  ;[1 1 1] counting the spll markers
  (if (`self.ActorHasTag` OtherActor "Player")
    (bind _asbp_blue_rov (cast `/Game/Blueprints/BP_BlueRov` (`GameplayStatics.GetPlayerPawn` 0)))
    (set `/Game/Blueprints/BP_BlueRov.SpecialCheckpointCount` (+ (`/Game/Blueprints/BP_BlueRov.SpecialCheckpointCount` _asbp_blue_rov) 1) _asbp_blue_rov)))

(fn `UserConstructionScript`)