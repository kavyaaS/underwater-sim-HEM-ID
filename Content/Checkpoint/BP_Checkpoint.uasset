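; BP_Checkpoint is a numbered checkpoint actor with a torus mesh that BP_BlueRov clears by passing through it.
; When the ROV stops overlapping the Trigger, it broadcasts CheckpointCleared with its CheckpointNumber, hides the trigger and torus, and destroys itself.
; A velocity-versus-Arrow direction check is present but unused, so exiting from either side counts.
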(event `self.Trigger.OnComponentEndOverlap`
  (params (OverlappedComponent :type "PrimitiveComponent Object Reference") (OtherActor :type "Actor Object Reference") (OtherComp :type "PrimitiveComponent Object Reference") (OtherBodyIndex :type Integer))
  (bind _trigger (`self.Trigger`))
  ;[1 1 1] Checkpoint System Algo for Overlapping
  (bind _asbp_blue_rov (cast `/Game/Blueprints/BP_BlueRov` OtherActor))
  (`self.CheckpointCleared` (`self.CheckpointNumber`))
  (`SceneComponent.SetHiddenInGame` _trigger true true)
  (`SceneComponent.SetHiddenInGame` (`self.Torus_Checkpoint`) true true)
  (`self.K2_DestroyActor`)
  (set `PrimitiveComponent.bGenerateOverlapEvents` true _trigger :!enabledstate Disabled))

(fn `UserConstructionScript`)