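; Player controller for a BlueROV game, with scaffolding for lap and checkpoint racing.
; On BeginPlay it creates the HUD widget, adds it to the viewport and caches the player pawn as a BP_BlueRov reference.
; InitText converts velocity and checkpoint counts to text, though nothing here calls it.
; Race, timer, respawn, goal and save/load events and functions are empty stubs.
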(event `self.ReceiveBeginPlay`
  ;[1 1 1] Initialization and Getting References
  (bind _returnvalue (`|CreateWidget` "/Game/Blueprints/UI/HUD.HUD_C"))
  (bind _output_get (set `self.HUDReference` _returnvalue))
  (`UserWidget.AddToViewport` _output_get 0)
  (bind _asbp_blue_rov (cast `/Game/Blueprints/BP_BlueRov` (`GameplayStatics.GetPlayerPawn` 0)))
  (set `self.As BP Blue Rov Reference` _asbp_blue_rov))

(event `StartGameSetup`)

(event `Restart`)

(event `UpdateLap`)

(event `RespawnVehicle`)

(event `StartRaceTime`)

(event `StopRaceEvent`)

(event `StartLapTime`)

(event `StopLapTime`)

(fn `InitText`
  ;[1 1 1] Numerical Value Conversion to Text
  (set `self.VelocityText` (`KismetTextLibrary.Conv_IntToText` (`self.Velocity`)))
  (set `self.TotalCheckpointsText` (`KismetTextLibrary.Conv_IntToText` (`self.TotalCheckpoints`)))
  (set `self.PassedCheckpointsText` (`KismetTextLibrary.Conv_IntToText` (`self.PassedCheckpoints`))))

(fn `LapTimeCheck`)

(fn `LoadTheGame`)

(fn `RaceTimeCheck`)

(fn `SaveGameCheck`)

(fn `SaveTheGame`)

(fn `UpdateGoals`)

(fn `UserConstructionScript`)