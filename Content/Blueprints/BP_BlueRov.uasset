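; Player-controlled BlueROV vehicle for a timed checkpoint game, with a first-person camera toggle, minimap and score from normal plus special checkpoints.
; Interpolated axis inputs set speeds that Tick turns into swept movement, yaw and speed-based pitch and roll.
; Tick also runs a delay-based countdown that opens the end-game widget at zero.
; Number keys trigger HUD error, mitigation and control-handback notifications; other player and wizard inputs only print debug labels.
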(event `Key|Three`
  (params (Key :type "Key Structure"))
  ;[1 1 1] key pressed notification in hud
  (:`Pressed`
    (bind _asnew_hud (cast `/Game/Blueprints/NewHUD` (`PlayerController.GetHUD` (`GameplayStatics.GetPlayerController` 0))))
    (`/Game/MinimapWidgets/WB_UIForNotification.SplMarker Error Detected` (`/Game/Blueprints/NewHUD.UI ref` _asnew_hud))))

(event `Key|Five`
  (params (Key :type "Key Structure"))
  ;[1 1 1] key pressed notification in hud
  (:`Pressed`
    (bind _asnew_hud (cast `/Game/Blueprints/NewHUD` (`PlayerController.GetHUD` (`GameplayStatics.GetPlayerController` 0))))
    (`/Game/MinimapWidgets/WB_UIForNotification.Fish Error Detected` (`/Game/Blueprints/NewHUD.UI ref` _asnew_hud))))

(event `Key|Two`
  (params (Key :type "Key Structure"))
  ;[1 1 1] key pressed notification in hud
  (:`Pressed`
    (bind _asnew_hud (cast `/Game/Blueprints/NewHUD` (`PlayerController.GetHUD` (`GameplayStatics.GetPlayerController` 0))))
    (`/Game/MinimapWidgets/WB_UIForNotification.Decision Error Mitigated` (`/Game/Blueprints/NewHUD.UI ref` _asnew_hud))))

(event `self.ReceiveBeginPlay`
  (bind _returnvalue (`GameplayStatics.GetPlayerController` 0))
  ;[1 1 1] minimap widget
  (`|ExecutionSequence`
    (:`then_1`
      (`self.EnableInput` _returnvalue)
      (bind _returnvalue_2 (`|CreateWidget` "/Game/MinimapWidgets/WB_minimap.WB_minimap_C" _returnvalue))
      (`UserWidget.AddToViewport` _returnvalue_2 0))))

(event `Key|Zero`
  (params (Key :type "Key Structure"))
  ;[1 1 1] key pressed notification in hud
  (:`Pressed`
    (bind _asnew_hud (cast `/Game/Blueprints/NewHUD` (`PlayerController.GetHUD` (`GameplayStatics.GetPlayerController` 0))))
    (`/Game/MinimapWidgets/WB_UIForNotification.Giving Back Control` (`/Game/Blueprints/NewHUD.UI ref` _asnew_hud))))

(event `InputAction|View_Change`
  (params (Key :type "Key Structure"))
  ;[1 1 1] POV Control Algo
  (:`Pressed`
    (`ActorComponent.SetActive` (`self.CameraFP`) false false)
    (`ActorComponent.SetActive` (`self.Camera`) false false)
    (switch `int` (`self.CameraIndex`)
      (:`0`
        (set `self.CameraIndex` 1))
      (:`1`
        (set `self.CameraIndex` 0)))
    (`ActorComponent.SetActive` (select `int` (`self.CameraIndex`) :`0` (`self.Camera`) :`1` (`self.CameraFP`) :!type "ActorComponent Object Reference") true false)))

(event `Key|Four`
  (params (Key :type "Key Structure"))
  ;[1 1 1] key pressed notification in hud
  (:`Pressed`
    (bind _asnew_hud (cast `/Game/Blueprints/NewHUD` (`PlayerController.GetHUD` (`GameplayStatics.GetPlayerController` 0))))
    (`/Game/MinimapWidgets/WB_UIForNotification.SplMarker Error Mitigated` (`/Game/Blueprints/NewHUD.UI ref` _asnew_hud))))

(event `Key|Six`
  (params (Key :type "Key Structure"))
  ;[1 1 1] key pressed notification in hud
  (:`Pressed`
    (bind _asnew_hud (cast `/Game/Blueprints/NewHUD` (`PlayerController.GetHUD` (`GameplayStatics.GetPlayerController` 0))))
    (`/Game/MinimapWidgets/WB_UIForNotification.Fish Error Mitigated` (`/Game/Blueprints/NewHUD.UI ref` _asnew_hud))))

(event `Key|One`
  (params (Key :type "Key Structure"))
  ;[1 1 1] key pressed notification in hud
  (:`Pressed`
    (bind _asnew_hud (cast `/Game/Blueprints/NewHUD` (`PlayerController.GetHUD` (`GameplayStatics.GetPlayerController` 0))))
    (`/Game/MinimapWidgets/WB_UIForNotification.Decision Error Detected` (`/Game/Blueprints/NewHUD.UI ref` _asnew_hud))))

(event `self.ReceiveEndPlay`
  (params (EndPlayReason :type "EEndPlayReason Enum" :default "Destroyed"))
  (`|ExecutionSequence`
    (:`then_0`
      (`KismetSystemLibrary.PrintString` "normal checkpoint count")
      (`KismetSystemLibrary.PrintString` (`KismetStringLibrary.Conv_IntToString` (`self.CurrentCheckpoint`))))
    (:`then_1`
      (`KismetSystemLibrary.PrintString` "Spl Checkpoint count")
      (`KismetSystemLibrary.PrintString` (`KismetStringLibrary.Conv_IntToString` (`self.SpecialCheckpointCount`))))
    (:`then_2`
      (`KismetSystemLibrary.PrintString` "Score is")
      (`KismetSystemLibrary.PrintString` (`KismetStringLibrary.Conv_IntToString` (stale `self.ReceiveTick` _output_get_2))))))

(event `Key|Gamepad_LeftStick_Up`
  (params (Key :type "Key Structure"))
  ;[1 1 1] Player input print
  (:`Pressed`
    (`KismetSystemLibrary.PrintString` "Forward Motion")))

(event `Key|W`
  (params (Key :type "Key Structure"))
  ;[1 1 1] Wizard input parameters print
  (:`Pressed`
    (`KismetSystemLibrary.PrintString` "Robot Up")))

(event `Key|Right`
  (params (Key :type "Key Structure"))
  ;[1 1 1] Wizard input parameters print
  (:`Pressed`
    (`KismetSystemLibrary.PrintString` "Robot right")))

(event `Key|S`
  (params (Key :type "Key Structure"))
  ;[1 1 1] Wizard input parameters print
  (:`Pressed`
    (`KismetSystemLibrary.PrintString` "Robot down" :!label _label)))

(event `Key|Left`
  (params (Key :type "Key Structure"))
  ;[1 1 1] Wizard input parameters print
  (:`Pressed`
    (`KismetSystemLibrary.PrintString` "Robot left")))

(event `Key|Gamepad_LeftStick_Down`
  (params (Key :type "Key Structure"))
  ;[1 1 1] Player input print
  (:`Pressed`
    (`KismetSystemLibrary.PrintString` "Backward motion")))

(event `Key|Enter`
  (params (Key :type "Key Structure"))
  ;[1 1 1] Wizard input parameters print
  (:`Pressed`
    (goto _label)))

(event `self.ReceiveTick`
  (params (DeltaSeconds :type "Float (single-precision)"))
  (bind (_returnvalue_roll _returnvalue_pitch _returnvalue_yaw) (`KismetMathLibrary.BreakRotator` (`self.K2_GetActorRotation`)))
  ;[1 1 1] event tick duplicate
  (`|ExecutionSequence`
    (:`then_0`
      ;[1 1 1] minutes and seconds display
      (`KismetSystemLibrary.Delay` 1.0)
      (if (== (`self.Seconds`) 0)
        (if (== (`self.Minutes`) 0)
          (bind _returnvalue (`|CreateWidget` "/Game/MinimapWidgets/WB_EndGameDisplay.WB_EndGameDisplay_C"))
          (`UserWidget.AddToViewport` _returnvalue 0)
          (`KismetSystemLibrary.QuitGame` null "Quit" :!enabledstate Disabled)
          (else
            (set `self.Seconds` 59)
            (set `self.Minutes` (- (`self.Minutes`) 1))))
        (else
          (set `self.Seconds` (- (`self.Seconds`) 1)))))
    (:`then_1`
      ;[1 1 1] Overall Vehicle Dynamics Manager
      (bind _output_get (set `self.DeltaLocation` (* (+ (`KismetMathLibrary.ProjectVectorOnToPlane` (+ (* (`self.GetActorForwardVector`) (`self.FBSpeed`)) (* (`self.GetActorRightVector`) (`self.RLSpeed`))) (0.0 0.0 1.0)) (* (`self.GetActorUpVector`) (`self.UDSpeed`))) (`GameplayStatics.GetWorldDeltaSeconds`))))
      (`self.K2_AddActorWorldOffset` _output_get true)
      (`self.K2_SetActorRotation` (`KismetMathLibrary.MakeRotator` (* (`self.RLSpeed`) (`self.RLSpeedToRollFactor`)) (* (`self.FBSpeed`) (`self.FBSpeedToPitchFactor`)) (+ _returnvalue_yaw (* (`self.YawRotSpeed`) (`GameplayStatics.GetWorldDeltaSeconds`))))))
    (:`then_2`
      ;[1 1 1] Total Score Calculation for end game display
      (bind _output_get_2 (set `self.Score` (+ (`self.CurrentCheckpoint`) (`self.SpecialCheckpointCount`)))))))

(event `Key|Gamepad_RightStick_Right`
  (params (Key :type "Key Structure"))
  ;[1 1 1] Player input print
  (:`Pressed`
    (`KismetSystemLibrary.PrintString` "Right tilt")))

(event `Key|Up`
  (params (Key :type "Key Structure"))
  ;[1 1 1] Wizard input parameters print
  (:`Pressed`
    (`KismetSystemLibrary.PrintString` "Robot forward")))

(event `Key|Down`
  (params (Key :type "Key Structure"))
  ;[1 1 1] Wizard input parameters print
  (:`Pressed`
    (`KismetSystemLibrary.PrintString` "Robot backward" :!label _label_2)))

(event `Key|Gamepad_RightStick_Left`
  (params (Key :type "Key Structure"))
  ;[1 1 1] Player input print
  (:`Pressed`
    (`KismetSystemLibrary.PrintString` "Left tilt")))

(event `Key|SpaceBar`
  (params (Key :type "Key Structure"))
  ;[1 1 1] Wizard input parameters print
  (:`Pressed`
    (goto _label_2)))

(event `Key|Gamepad_Special_Right`
  (params (Key :type "Key Structure"))
  ;[1 1 1] Wizard input parameters print
  (:`Pressed`
    (`KismetSystemLibrary.PrintString` "Game Start")))

(event `Key|Gamepad_RightStick_Up`
  (params (Key :type "Key Structure"))
  ;[1 1 1] Player input print
  (:`Pressed`
    (`KismetSystemLibrary.PrintString` "Going up")))

(event `Key|Gamepad_Special_Left`
  (params (Key :type "Key Structure"))
  ;[1 1 1] Wizard input parameters print
  (:`Pressed`
    (`KismetSystemLibrary.PrintString` "Game End")))

(event `Key|Gamepad_RightStick_Down`
  (params (Key :type "Key Structure"))
  ;[1 1 1] Player input print
  (:`Pressed`
    (`KismetSystemLibrary.PrintString` "Going down")))

(event `Key|Gamepad_LeftStick_Right`
  (params (Key :type "Key Structure"))
  ;[1 1 1] Player input print
  (:`Pressed`
    (`KismetSystemLibrary.PrintString` "Turning right")))

(event `Key|Gamepad_LeftStick_Left`
  (params (Key :type "Key Structure"))
  ;[1 1 1] Player input print
  (:`Pressed`
    (`KismetSystemLibrary.PrintString` "Turning left")))

(event `InputAxis|ForwardBackward`
  (params (AxisValue :type "Float (single-precision)"))
  ;[1 1 1] Forward Backward Dynamics
  (set `self.FBSpeed` (`KismetMathLibrary.FInterpTo` (`self.FBSpeed`) (* AxisValue (`self.FBSpeedFactor`)) (`GameplayStatics.GetWorldDeltaSeconds`) 2.0)))

(event `InputAxis|RightLeft`
  (params (AxisValue :type "Float (single-precision)"))
  ;[1 1 1] Right Left Dynamics
  (set `self.RLSpeed` (`KismetMathLibrary.FInterpTo` (`self.RLSpeed`) (* AxisValue (`self.RLSpeedFactor`)) (`GameplayStatics.GetWorldDeltaSeconds`) 2.0)))

(event `InputAxis|UpDown`
  (params (AxisValue :type "Float (single-precision)"))
  ;[1 1 1] Up Down Dynamics
  (set `self.UDSpeed` (`KismetMathLibrary.FInterpTo` (`self.UDSpeed`) (* AxisValue (`self.UDSpeedFactor`)) (`GameplayStatics.GetWorldDeltaSeconds`) 2.0)))

(event `InputAxis|YawRotation`
  (params (AxisValue :type "Float (single-precision)"))
  ;[1 1 1] Yaw Rotation Dynamics
  (set `self.YawRotSpeed` (`KismetMathLibrary.FInterpTo` (`self.YawRotSpeed`) (* AxisValue (`self.YawRotSpeedFactor`)) (`GameplayStatics.GetWorldDeltaSeconds`) 2.0)))

(event `self.SphereCollision.OnComponentBeginOverlap`
  (params (OverlappedComponent :type "PrimitiveComponent Object Reference") (OtherActor :type "Actor Object Reference") (OtherComp :type "PrimitiveComponent Object Reference") (OtherBodyIndex :type Integer) (bFromSweep :type Boolean) (SweepResult :type "HitResult Structure (by ref)"))
  ;[1 1 1] Collition_detection
  (`KismetSystemLibrary.PrintString` (`KismetSystemLibrary.GetDisplayName` OtherActor)))

(fn `UserConstructionScript`)