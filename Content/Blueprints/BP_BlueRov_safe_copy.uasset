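; Player-controlled BlueRov vehicle pawn that moves on four axes, with a minimap widget and a toggle between two cameras.
; Axis inputs ease forward, lateral, vertical and yaw speeds toward scaled targets using FInterpTo.
; Tick applies a swept offset, flattening forward and lateral motion to the horizontal plane, and derives cosmetic-style roll and pitch from speed while integrating yaw.
; Sphere overlaps only print the other actor's name.
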(event `InputAction|View_Change`
  (params (Key :type "Key Structure"))
  ;[1 1 1] POV Control Algo
  (:`Pressed`
    (`ActorComponent.SetActive` (`self.CameraFP`) false false)
    (`ActorComponent.SetActive` (`self.Camera`) false false)
    (switch `int` (`self.CameraIndex`)
      (:`0`
        (set `self.CameraIndex` 1))
      (:`1`
        (set `self.CameraIndex` 0)))
    (`ActorComponent.SetActive` (select `int` (`self.CameraIndex`) :`0` (`self.Camera`) :`1` (`self.CameraFP`) :!type "ActorComponent Object Reference") true false)))

(event `self.ReceiveBeginPlay`
  (bind _returnvalue (`|CreateWidget` "/Game/MinimapWidgets/WB_minimap.WB_minimap_C" (`GameplayStatics.GetPlayerController` 0)))
  (`UserWidget.AddToViewport` _returnvalue 0))

(event `self.ReceiveTick`
  (params (DeltaSeconds :type "Float (single-precision)"))
  (bind (_returnvalue_roll _returnvalue_pitch _returnvalue_yaw) (`KismetMathLibrary.BreakRotator` (`self.K2_GetActorRotation`)))
  ;[1 1 1] Overall Vehicle Dynamics Manager
  (bind _output_get (set `self.DeltaLocation` (* (+ (`KismetMathLibrary.ProjectVectorOnToPlane` (+ (* (`self.GetActorForwardVector`) (`self.FBSpeed`)) (* (`self.GetActorRightVector`) (`self.RLSpeed`))) (0.0 0.0 1.0)) (* (`self.GetActorUpVector`) (`self.UDSpeed`))) (`GameplayStatics.GetWorldDeltaSeconds`))))
  (`self.K2_AddActorWorldOffset` _output_get true)
  (`self.K2_SetActorRotation` (`KismetMathLibrary.MakeRotator` (* (`self.RLSpeed`) (`self.RLSpeedToRollFactor`)) (* (`self.FBSpeed`) (`self.FBSpeedToPitchFactor`)) (+ _returnvalue_yaw (* (`self.YawRotSpeed`) (`GameplayStatics.GetWorldDeltaSeconds`))))))

(event `InputAxis|ForwardBackward`
  (params (AxisValue :type "Float (single-precision)"))
  ;[1 1 1] Forward Backward Dynamics
  (set `self.FBSpeed` (`KismetMathLibrary.FInterpTo` (`self.FBSpeed`) (* AxisValue (`self.FBSpeedFactor`)) (`GameplayStatics.GetWorldDeltaSeconds`) 2.0)))

(event `InputAxis|RightLeft`
  (params (AxisValue :type "Float (single-precision)"))
  ;[1 1 1] Right Left Dynamics
  (set `self.RLSpeed` (`KismetMathLibrary.FInterpTo` (`self.RLSpeed`) (* AxisValue (`self.RLSpeedFactor`)) (`GameplayStatics.GetWorldDeltaSeconds`) 2.0)))

(event `InputAxis|UpDown`
  (params (AxisValue :type "Float (single-precision)"))
  ;[1 1 1] Up Down Dynamics
  (set `self.UDSpeed` (`KismetMathLibrary.FInterpTo` (`self.UDSpeed`) (* AxisValue (`self.UDSpeedFactor`)) (`GameplayStatics.GetWorldDeltaSeconds`) 2.0)))

(event `InputAxis|YawRotation`
  (params (AxisValue :type "Float (single-precision)"))
  ;[1 1 1] Yaw Rotation Dynamics
  (set `self.YawRotSpeed` (`KismetMathLibrary.FInterpTo` (`self.YawRotSpeed`) (* AxisValue (`self.YawRotSpeedFactor`)) (`GameplayStatics.GetWorldDeltaSeconds`) 2.0)))

(event `self.SphereCollision.OnComponentBeginOverlap`
  (params (OverlappedComponent :type "PrimitiveComponent Object Reference") (OtherActor :type "Actor Object Reference") (OtherComp :type "PrimitiveComponent Object Reference") (OtherBodyIndex :type Integer) (bFromSweep :type Boolean) (SweepResult :type "HitResult Structure (by ref)"))
  ;[1 1 1] Collition_detection
  (`KismetSystemLibrary.PrintString` (`KismetSystemLibrary.GetDisplayName` OtherActor)))

(fn `UserConstructionScript`)